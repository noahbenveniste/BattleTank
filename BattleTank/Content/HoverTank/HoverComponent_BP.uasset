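; Hover component that acts as one suspension point on a hover tank, pushing the vehicle up off surfaces beneath it.
; Each tick it traces down its own up vector by HoverDistance and treats the shortfall to the hit as spring compression.
; A spring-damper force, damped by the change in compression over delta time, is applied to the parent's root primitive at the component's location.
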(event `self.ReceiveBeginPlay`
  ;[1 1 1] Set reference to parent vehicle
  (bind _ashover_tank_test_bp (cast `/Game/HoverTank/HoverTankTest_BP` (`self.GetOwner`)))
  (set `self.ParentVehicle` _ashover_tank_test_bp))

(event `self.ReceiveTick`
  (params (DeltaSeconds :type "Float (single-precision)"))
  (bind _returnvalue (`self.K2_GetComponentLocation`))
  ;[1 1 1] Hover only when the parent vehicle is valid
  (`/Engine/EditorBlueprintResources/StandardMacros.IsValid` (`self.ParentVehicle`)
    (:`Is Valid`
      (bind (_outhit _returnvalue_2) (`KismetSystemLibrary.LineTraceSingle` :`Start` _returnvalue :`End` (- _returnvalue (* (`self.GetUpVector`) (`self.HoverDistance`))) :`TraceChannel` "TraceTypeQuery1" :`DrawDebugType` "ForOneFrame"))
      (if _returnvalue_2
        ;[1 1 1] Calculate the HoverDelta, i.e. the compression/elongation of our "spring"
        (bind _output_get (set `self.HoverDelta` (- (`self.HoverDistance`) (`KismetMathLibrary.VSize` (- (`.Location` (`GameplayStatics.BreakHitResult` _outhit)) (`self.K2_GetComponentLocation`))))))
        (`PrimitiveComponent.AddForceAtLocation` (cast `PrimitiveComponent` (`Actor.RootComponent` (`self.ParentVehicle`)) :!pure true) (* (`self.GetUpVector`) (+ (* (/ (- _output_get (`self.PreviousHoverDelta`)) (`GameplayStatics.GetWorldDeltaSeconds`)) (`self.DampingCoefficient`)) (* _output_get (`self.SpringCoefficient`)))) (`self.K2_GetComponentLocation`) "None") ; Apply the force
        (set `self.PreviousHoverDelta` (`self.HoverDelta`)) ; Set the current HoverDelta to PreviousHoverDelta\nfor the next frame
      ))))