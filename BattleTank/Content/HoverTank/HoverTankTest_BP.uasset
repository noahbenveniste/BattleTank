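; Test hover tank Blueprint that the player drives with physics forces while orbiting an aim camera.
; W/S and A/D key events set forward force and turn torque values, zeroing them on release.
; Tick applies those values to TankBody0 along the actor's forward and up vectors; no hover lift is implemented in these graphs.
; AimAzimuth yaws AzimuthGimbal0 and AimElevation pitches SpringArm0, with no clamping.
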(event `InputAxis|AimAzimuth`
  (params (AxisValue :type "Float (single-precision)"))
  ;[1 1 1] Camera Input Binding
  (`SceneComponent.K2_AddLocalRotation` (`self.AzimuthGimbal_0`) (`KismetMathLibrary.MakeRotator` 0.0 0.0 AxisValue) false false))

(event `Key|W`
  (params (Key :type "Key Structure"))
  ;[1 1 1] Linear movement input bindings
  (:`Pressed`
    (set `self.ForwardForce` 50000.0))
  (:`Released`
    (set `self.ForwardForce` 0.0 :!label _label)))

(event `Key|D`
  (params (Key :type "Key Structure"))
  ;[1 1 1] Rotational movement input bindings. Torques are very large because in UE4 the base unit is cm
  (:`Pressed`
    (set `self.TurnTorque` 1000000.0))
  (:`Released`
    (set `self.TurnTorque` 0.0 :!label _label_2)))

(event `Key|S`
  (params (Key :type "Key Structure"))
  ;[1 1 1] Linear movement input bindings
  (:`Pressed`
    (set `self.ForwardForce` -50000.0))
  (:`Released`
    (goto _label)))

(event `Key|A`
  (params (Key :type "Key Structure"))
  ;[1 1 1] Rotational movement input bindings. Torques are very large because in UE4 the base unit is cm
  (:`Pressed`
    (set `self.TurnTorque` -1000000.0))
  (:`Released`
    (goto _label_2)))

(event `InputAxis|AimElevation`
  (params (AxisValue :type "Float (single-precision)"))
  ;[1 1 1] Camera Input Binding
  (`SceneComponent.K2_AddLocalRotation` (`self.SpringArm_0`) (`KismetMathLibrary.MakeRotator` 0.0 AxisValue) false false))

(event `self.ReceiveTick`
  (params (DeltaSeconds :type "Float (single-precision)"))
  (`PrimitiveComponent.AddForce` (`self.TankBody_0`) (* (`self.GetActorForwardVector`) (`self.ForwardForce`)) "None" false)
  (`PrimitiveComponent.AddTorque` (`self.TankBody_0`) (* (`self.GetActorUpVector`) (`self.TurnTorque`)) "None" false))

(fn `UserConstructionScript`)